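; BP_Vehicle1 is a player-driven hover vehicle pawn that adds its Enhanced Input mapping on BeginPlay.
; Thrust works only while the hover component reports a hit, setting the movement component's target speed and scaling thruster volume and pitch.
; Turn drives target angular speed, while Boost raises max speed for later thrust input and restores it only on Canceled, not Completed.
; Hits play an attenuated impact sound at the contact point.
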(event Input|EnhancedActionEvents|EnhancedInputActionThrust
  (params (ActionValue :type Float%20%28double-precision%29) (ElapsedSeconds :type Float%20%28double-precision%29) (TriggeredSeconds :type Float%20%28double-precision%29) (InputAction :type Input%20Action%20Object%20Reference :default "/Game/Controls/Thrust.Thrust"))
  (bind _thrustersound (Variables|Default|Getthrustersound))
  (if (Variables|/Game/Blueprints/PhysicsComponents/SC_HoverComponent.SC_HoverComponent_C|Getis%20hit (Variables|Default|GetSC_HoverComponent2))
    (Variables|/Game/Blueprints/PhysicsComponents/AC_MovementComponent.AC_MovementComponent_C|SetTargetSpeed (Variables|Default|GetAC_MovementComponent) (* ActionValue (Variables|Default|GetMaxSpeed)))
    (Audio|Components|Audio|SetVolumeMultiplier _thrustersound (* ActionValue 0.2) :!class /Script/Engine.AudioComponent)
    (Audio|Components|Audio|SetPitchMultiplier _thrustersound (* ActionValue 3.0))))

(event Input|EnhancedActionEvents|EnhancedInputActionTurn
  (params (ActionValue :type Float%20%28double-precision%29) (ElapsedSeconds :type Float%20%28double-precision%29) (TriggeredSeconds :type Float%20%28double-precision%29) (InputAction :type Input%20Action%20Object%20Reference :default "/Game/Controls/Turn.Turn"))
  (bind _ac_movementcomponent (Variables|Default|GetAC_MovementComponent))
  (:Triggered
    (Variables|/Game/Blueprints/PhysicsComponents/AC_MovementComponent.AC_MovementComponent_C|SetTargetAngularSpeed _ac_movementcomponent (* ActionValue (Variables|Default|GetSteerFactor))))
  (:Canceled
    (Variables|/Game/Blueprints/PhysicsComponents/AC_MovementComponent.AC_MovementComponent_C|SetTargetAngularSpeed _ac_movementcomponent 0.0 :!label _label))
  (:Completed
    (goto _label)))

(event Input|EnhancedActionEvents|EnhancedInputActionBoost
  (params (ActionValue :type Boolean) (ElapsedSeconds :type Float%20%28double-precision%29) (TriggeredSeconds :type Float%20%28double-precision%29) (InputAction :type Input%20Action%20Object%20Reference :default "/Game/Controls/Boost.Boost"))
  (:Triggered
    (Variables|Default|SetMaxSpeed 2.5e+03))
  (:Canceled
    (Variables|Default|SetMaxSpeed 2e+03)))

(event EventBeginPlay
  (bind _asplayer_controller (Utilities|Casting|CastToPlayerController (Pawn|GetController)))
  (Utilities|IsValid (PlayerController|LocalPlayerSubsystems|GetEnhancedInputLocalPlayerSubsystem _asplayer_controller)
    (:Is%20Valid
      (Input|AddMappingContext (PlayerController|LocalPlayerSubsystems|GetEnhancedInputLocalPlayerSubsystem _asplayer_controller) "/Game/Controls/GameControls.GameControls" 0 "(bIgnoreAllPressedKeysUntilRelease=True,bForceImmediately=False,bNotifyUserSettings=False)"))))

(event EventTick
  (params (DeltaSeconds :type Float%20%28single-precision%29)))

(event Collision|EventHit
  (params (MyComp :type Primitive%20Component%20Object%20Reference) (Other :type Actor%20Object%20Reference) (OtherComp :type Primitive%20Component%20Object%20Reference) (bSelfMoved :type Boolean) (HitLocation :type Vector :default "0, 0, 0") (HitNormal :type Vector :default "0, 0, 0") (NormalImpulse :type Vector :default "0, 0, 0") (Hit :type Hit%20Result%20Structure%20%28by%20ref%29))
  (Audio|PlaySoundatLocation "/Game/Sound/SoundEffects/Crash/VehicleImpactCue.VehicleImpactCue" HitLocation "0, 0, 0" 0.5 1.0 0.0 "/Game/Sound/SoundEffects/Attenuation/ImpactSounds.ImpactSounds" 0 0 0))

(fn ConstructionScript)