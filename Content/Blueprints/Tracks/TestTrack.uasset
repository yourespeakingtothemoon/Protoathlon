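; TestTrack is a track actor that builds its geometry from a spline in the construction script.
; It adds a collision-enabled spline mesh between each pair of neighboring points, matching their local positions and tangents.
; A closing segment back to the first point is always added, despite an "Only if Closed Loop" note, and simulates physics without gravity.
; The event graph is unused.
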(event EventBeginPlay)

(event Collision|EventActorBeginOverlap
  (params (OtherActor :type Actor%20Object%20Reference)))

(event EventTick
  (params (DeltaSeconds :type Float%20%28single-precision%29)))

(fn ConstructionScript
  (bind _spline (Variables|Default|GetSpline))
  (bind (_location _tangent) (Spline|GetLocationandTangentatSplinePoint _spline 0 "Local"))
  (for _index (range 0 (- (Spline|GetNumberOfSplinePoints (Variables|Default|GetSpline)) 2))
    (bind _returnvalue (AddComponent|AddSplineMeshComponent false))
    (Collision|SetCollisionEnabled _returnvalue "QueryAndPhysics")
    (SplineMesh|SetStartandEnd _returnvalue (.Location (Spline|GetLocationandTangentatSplinePoint (Variables|Default|GetSpline) _index "Local")) (.Tangent (Spline|GetLocationandTangentatSplinePoint (Variables|Default|GetSpline) _index "Local")) (.Location (Spline|GetLocationandTangentatSplinePoint (Variables|Default|GetSpline) (+ _index 1) "Local")) (.Tangent (Spline|GetLocationandTangentatSplinePoint (Variables|Default|GetSpline) (+ _index 1) "Local")) true :!class /Script/Engine.SplineMeshComponent)
    (Transformation|AttachComponentToComponent _returnvalue 0 "None" "KeepRelative" "KeepRelative" "KeepRelative" true))
  ;[1 1 1] Only if Closed Loop
  (bind _returnvalue_2 (AddComponent|AddSplineMeshComponent false))
  (Physics|SetSimulatePhysics _returnvalue_2 true)
  (Physics|SetEnableGravity _returnvalue_2 false)
  (Collision|SetCollisionEnabled _returnvalue_2 "QueryAndPhysics")
  (SplineMesh|SetStartandEnd _returnvalue_2 (.Location (Spline|GetLocationandTangentatSplinePoint (Variables|Default|GetSpline) _index "Local")) (.Tangent (Spline|GetLocationandTangentatSplinePoint (Variables|Default|GetSpline) _index "Local")) _location _tangent true :!class /Script/Engine.SplineMeshComponent))