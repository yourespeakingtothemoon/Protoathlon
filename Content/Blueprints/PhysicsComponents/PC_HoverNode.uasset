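; PC_HoverNode is a hover node that makes its owner's physics-simulated primitive component float above surfaces below it.
; Each tick it traces straight down from its Sphere up to HoverDistance on the Visibility channel, with debug drawing.
; On a hit, it applies a spring-like force along the Sphere's up vector, fading linearly with distance.
; The force acts without a location offset, and hits also set linear and angular damping, which is never reset.
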(event EventBeginPlay
  (bind _output_get (Variables|Default|SetPrim (Actor|GetComponentbyClass (Components|GetOwner) "/Script/Engine.PrimitiveComponent")))
  (Physics|SetSimulatePhysics _output_get true))

(event Collision|EventActorBeginOverlap
  (params (OtherActor :type Actor%20Object%20Reference)))

(event EventTick
  (params (DeltaSeconds :type Float%20%28single-precision%29))
  (bind (_spring_force _hit) (CallFunction|Raycast))
  (if _hit
    (Physics|AddForce (Variables|Default|GetPrim) _spring_force "None" false)
    (Class|PrimitiveComponent|SetLinearDamping (Variables|Default|GetPrim) (Variables|Default|GetLinear%20Damping))
    (Class|PrimitiveComponent|SetAngularDamping (Variables|Default|GetPrim) (Variables|Default|GetAngular%20Damping))))

(fn ConstructionScript)

(fn Raycast
  (bind _sphere (Variables|Default|GetSphere))
  (bind _returnvalue (Transformation|GetWorldLocation _sphere))
  (bind (_outhit _returnvalue_2) (Collision|LineTraceByChannel (Transformation|GetWorldLocation (Variables|Default|GetSphere)) (Math|Vector|MakeVector (.x _returnvalue) (.y _returnvalue) (- (.z _returnvalue) (Variables|Default|GetHover%20Distance))) "TraceTypeQuery1" false 0 "ForDuration"))
  (return (* (Math|Float|Lerp (Variables|Default|GetForce) 0.0 (/ (.Distance (Collision|BreakHitResult _outhit)) (Variables|Default|GetHover%20Distance))) (Math|Vector|GetUpVector (Variables|Default|GetSphere))) _returnvalue_2))