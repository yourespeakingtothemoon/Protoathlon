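; AC_HoverComponent is an actor component that makes a physics primitive hover above surfaces.
; Each tick it line-traces straight down over the hover distance on the Visibility channel, with debug drawing on.
; On a hit, it pushes the primitive along the impact normal with a force fading linearly to zero at full distance, and applies linear and angular damping, which is not reset on a miss.
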(event EventBeginPlay)

(event EventTick
  (params (DeltaSeconds :type Float%20%28single-precision%29))
  (bind (_spring_force _hit) (CallFunction|GetSpringForce))
  (if _hit
    (Physics|AddForce (Variables|Default|GetPrim) _spring_force "None" false)
    (Class|PrimitiveComponent|SetLinearDamping (Variables|Default|GetPrim) (Variables|Default|GetLinear%20Damping))
    (Class|PrimitiveComponent|SetAngularDamping (Variables|Default|GetPrim) (Variables|Default|GetAngular%20Damping))))

(fn GetSpringForce
  (bind _location (Variables|Default|GetLocation))
  (bind (_outhit _returnvalue) (Collision|LineTraceByChannel (Variables|Default|GetLocation) (Math|Vector|MakeVector (.x _location) (.y _location) (- (.z _location) (Variables|Default|GetHover%20Distance))) "TraceTypeQuery1" false 0 "ForDuration"))
  (Variables|Default|Sethit%20info _outhit)
  (return (* (Math|Float|Lerp (Variables|Default|GetForce) 0.0 (/ (.Distance (Collision|BreakHitResult _outhit)) (Variables|Default|GetHover%20Distance))) (.ImpactNormal (Collision|BreakHitResult _outhit))) _returnvalue))