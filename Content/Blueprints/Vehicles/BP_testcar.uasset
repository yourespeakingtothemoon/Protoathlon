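; Prototype hover car that floats above the ground using a physics force on its Testcaragain component.
; Each Tick, Hover traces downward with debug drawing and applies upward acceleration, switching between two values near gravity strength based on ground distance.
; Throttle, steering, transform-based movement and sine-offset helpers are defined but not called in this graph; Hop and Boost are empty stubs.
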(event EventBeginPlay)

(event Collision|EventActorBeginOverlap
  (params (OtherActor :type Actor%20Object%20Reference)))

(event EventTick
  (params (DeltaSeconds :type Float%20%28single-precision%29))
  (CallFunction|Hover 9.0 982.0 DeltaSeconds))

(fn ConstructionScript)

(fn Hover
  (params (Hover%20Distance :type Float%20%28double-precision%29) (Force%20Intesnsity :type Float%20%28double-precision%29) (deltaTime :type Float%20%28double-precision%29))
  (bind _distance (CallFunction|CastRayDown))
  (Physics|AddForce (Variables|Default|Gettestcaragain) (Math|Vector|MakeVector 0.0 0.0 (Math|Float|SelectFloat Force%20Intesnsity 975.0 (< _distance Hover%20Distance))) "None" true))

(fn CastRayDown
  (bind _returnvalue (Transformation|GetActorLocation))
  (bind (_outhit _returnvalue_2) (Collision|LineTraceByChannel _returnvalue (- _returnvalue "0.000000,0.000000,2000.000000") "TraceTypeQuery2" false 0 "ForDuration"))
  (if _returnvalue_2
    (return (.Distance (Collision|BreakHitResult _outhit)) (.z (.Location (Collision|BreakHitResult _outhit))))
    (else
      (return 1e+04 0.0))))

(fn Sineify
  (params (Intensity :type Float%20%28double-precision%29) (InHoverPosit :type Float%20%28double-precision%29) (deltaTime :type Float%20%28double-precision%29))
  (bind _result (CallFunction|SineOffset 1e+01 deltaTime))
  (return (+ (* _result Intensity) InHoverPosit)))

(fn SineOffset
  (params (Frequency :type Float%20%28double-precision%29) (Delta%20Time :type Float%20%28double-precision%29))
  (return (* 2.0 (Math|Trig|GetPI) Frequency Delta%20Time)))

(fn Throttle
  (params (Throttle%20Amount :type Float%20%28double-precision%29) (Max%20Speed :type Float%20%28double-precision%29))
  (return (Math|Interpolation|FInterpTo (Variables|Default|GetCurrent%20Speed) (* Throttle%20Amount Max%20Speed) (Utilities|Time|GetWorldDeltaSeconds) 4.0)))

(fn UpdateSteering
  (params (DeltaTime :type Float%20%28double-precision%29) (Speed :type Float%20%28double-precision%29) (SteerAngle :type Float%20%28double-precision%29) (Steer%20Response%20Factor :type Float%20%28double-precision%29))
  (Class|Actor|AddActorWorldRotation (Math|Rotator|MakeRotator 0.0 0.0 (* Speed SteerAngle Steer%20Response%20Factor))))

(fn Hop)

(fn Boost)

(fn UpdateMovement
  (params (DeltaTime :type Float%20%28double-precision%29) (Speed :type Float%20%28double-precision%29))
  (Transformation|AddActorWorldOffset (* DeltaTime (* Speed (Transformation|GetActorForwardVector)))))

(fn Steer
  (params (Axis%20Value :type Float%20%28double-precision%29))
  (return (Math|Interpolation|FInterpTo (Variables|Default|GetSteer%20Angle) (* Axis%20Value (Variables|Default|GetTurn%20Stat)) (Utilities|Time|GetWorldDeltaSeconds) 4.0)))