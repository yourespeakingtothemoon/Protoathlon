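; AC_LatStabilizer is an actor component that damps sideways sliding of its owner's physics body.
; On BeginPlay it caches the owner's root component as a primitive body reference.
; Each tick it projects linear velocity onto the body's right vector and applies an opposing force along that axis, scaled by SpeedToForce.
; The force is mass-dependent rather than an acceleration change.
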(event EventBeginPlay
  (bind _asprimitive_component (Utilities|Casting|CastToPrimitiveComponent (Variables|/Script/Engine.Actor|GetRootComponent (Components|GetOwner))))
  (Variables|Default|SetBodyRef _asprimitive_component))

(event EventTick
  (params (DeltaSeconds :type Float%20%28single-precision%29))
  (bind _bodyref (Variables|Default|GetBodyRef))
  (bind _bodyref_2 (Variables|Default|GetBodyRef)
    (:then
      (bind _returnvalue (Physics|GetPhysicsLinearVelocity _bodyref_2 "None"))
      (Physics|AddForce _bodyref (* (Math|Vector|GetRightVector _bodyref) (* (Math|Vector|DotProduct _returnvalue (Math|Vector|GetRightVector _bodyref_2)) -1.0 (Variables|Default|GetSpeedToForce))) "None" false))
    (:else)))