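; Player-driven hover vehicle pawn with throttle, brake, e-brake and a depletable boost via Enhanced Input.
; Inputs ease speed and steer angle with FInterpTo; Tick applies them as transform changes, plus air resistance.
; A downward trace sets hover height, steering rolls the mesh (harder when e-braking), and optional steer assist pulls yaw toward the TestTrack spline.
; Boost amount and e-brake "Sparks!" are only debug prints.
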(event Input|EnhancedActionEvents|EnhancedInputActionThrust
  (params (ActionValue :type Float%20%28double-precision%29) (ElapsedSeconds :type Float%20%28double-precision%29) (TriggeredSeconds :type Float%20%28double-precision%29) (InputAction :type Input%20Action%20Object%20Reference :default "/Game/Controls/Thrust.Thrust"))
  (bind _speed (CallFunction|Throttle ActionValue (Variables|Default|GetMax%20Speed)))
  (Variables|Default|SetCurrent%20Speed _speed))

(event Input|EnhancedActionEvents|EnhancedInputActionTurn
  (params (ActionValue :type Float%20%28double-precision%29) (ElapsedSeconds :type Float%20%28double-precision%29) (TriggeredSeconds :type Float%20%28double-precision%29) (InputAction :type Input%20Action%20Object%20Reference :default "/Game/Controls/Turn.Turn"))
  (:Triggered
    (bind _steer_angle (CallFunction|Steer ActionValue :!label _label))
    (Variables|Default|SetCurrent%20Steer%20Angle _steer_angle))
  (:Canceled
    (goto _label)))

(event Input|EnhancedActionEvents|EnhancedInputActionBrake
  (params (ActionValue :type Float%20%28double-precision%29) (ElapsedSeconds :type Float%20%28double-precision%29) (TriggeredSeconds :type Float%20%28double-precision%29) (InputAction :type Input%20Action%20Object%20Reference :default "/Game/Controls/Brake.Brake"))
  (bind _speed (CallFunction|Throttle (* ActionValue -0.5) (Variables|Default|GetMax%20Speed)))
  (Variables|Default|SetCurrent%20Speed _speed))

(event Input|EnhancedActionEvents|EnhancedInputActionEBrake
  (params (ActionValue :type Float%20%28double-precision%29) (ElapsedSeconds :type Float%20%28double-precision%29) (TriggeredSeconds :type Float%20%28double-precision%29) (InputAction :type Input%20Action%20Object%20Reference :default "/Game/Controls/EBrake.EBrake"))
  (:Triggered
    (Variables|Default|SetCurrent%20Speed (Math|Interpolation|FInterpTo (Variables|Default|GetCurrent%20Speed) 0.0 (Utilities|Time|GetWorldDeltaSeconds) 5.0) :!label _label)
    (Variables|Default|SetTiltDenom 2.0))
  (:Started
    (goto _label))
  (:Canceled
    (Variables|Default|SetTiltDenom 6.0 :!label _label_2))
  (:Completed
    (goto _label_2)))

(event Input|EnhancedActionEvents|EnhancedInputActionBoost
  (params (ActionValue :type Boolean) (ElapsedSeconds :type Float%20%28double-precision%29) (TriggeredSeconds :type Float%20%28double-precision%29) (InputAction :type Input%20Action%20Object%20Reference :default "/Game/Controls/Boost.Boost"))
  (:Triggered
    (Development|PrintText (Utilities|Text|ToText(Float) (Variables|Default|GetRemaining%20Boost) "HalfToEven") true true "(R=0.120321,G=0.126944,B=1.000000,A=1.000000)" :!label _label)
    (if (> (Variables|Default|GetRemaining%20Boost) 0.0)
      (Variables|Default|SetRemaining%20Boost (- (Variables|Default|GetRemaining%20Boost) 0.1))
      (Variables|Default|SetCurrent%20Speed (Math|Interpolation|FInterpTo (Variables|Default|GetCurrent%20Speed) (* (Variables|Default|GetMax%20Speed) 3.0) (Utilities|Time|GetWorldDeltaSeconds) 6.0))))
  (:Ongoing
    (goto _label)))

(event EventBeginPlay
  (bind _asplayer_controller (Utilities|Casting|CastToPlayerController (Pawn|GetController)))
  (Utilities|IsValid (PlayerController|LocalPlayerSubsystems|GetEnhancedInputLocalPlayerSubsystem _asplayer_controller)
    (:Is%20Valid
      (Input|AddMappingContext (PlayerController|LocalPlayerSubsystems|GetEnhancedInputLocalPlayerSubsystem _asplayer_controller) "/Game/Controls/GameControls.GameControls" 0 "(bIgnoreAllPressedKeysUntilRelease=True,bForceImmediately=False,bNotifyUserSettings=False)")
      (bind _returnvalue (Actor|GetActorOfClass "/Game/Blueprints/Tracks/TestTrack.TestTrack_C"))
      (Variables|Default|SetSpline _returnvalue))))

(event Collision|EventActorBeginOverlap
  (params (OtherActor :type Actor%20Object%20Reference)))

(event EventTick
  (params (DeltaSeconds :type Float%20%28single-precision%29))
  (bind _current_speed (Variables|Default|GetCurrent%20Speed))
  (CallFunction|Hover 15.0 982.0 DeltaSeconds)
  (CallFunction|UpdateMovement DeltaSeconds _current_speed)
  (CallFunction|UpdateSteering DeltaSeconds _current_speed (Variables|Default|GetCurrent%20Steer%20Angle) (Variables|Default|GetSRFactor))
  (CallFunction|AirResist))

(fn ConstructionScript)

(fn Throttle
  (params (Throttle%20Amount :type Float%20%28double-precision%29) (Max%20Speed :type Float%20%28double-precision%29))
  (return (Math|Interpolation|FInterpTo (Variables|Default|GetCurrent%20Speed) (* Throttle%20Amount Max%20Speed) (Utilities|Time|GetWorldDeltaSeconds) 4.0)))

(fn UpdateSteering
  (params (DeltaTime :type Float%20%28double-precision%29) (Speed :type Float%20%28double-precision%29) (SteerAngle :type Float%20%28double-precision%29) (Steer%20Response%20Factor :type Float%20%28double-precision%29))
  (CallFunction|SteerTilt SteerAngle)
  (Class|Actor|AddActorWorldRotation (Math|Rotator|MakeRotator 0.0 0.0 (* DeltaTime SteerAngle Steer%20Response%20Factor)))
  (if (Variables|Default|GetSteerAssist)
    (CallFunction|BindYaw 4.0)))

(fn UpdateMovement
  (params (DeltaTime :type Float%20%28double-precision%29) (Speed :type Float%20%28double-precision%29))
  (Transformation|AddActorWorldOffset (* Speed (Math|Vector|GetForwardVector (Variables|Default|Gettestcaragain)) DeltaTime)))

(fn Steer
  (params (Axis%20Value :type Float%20%28double-precision%29))
  (return (Math|Interpolation|FInterpTo (Variables|Default|GetCurrent%20Steer%20Angle) (* Axis%20Value (Variables|Default|GetSteer%20Stat)) (Utilities|Time|GetWorldDeltaSeconds) 4.0)))

(fn CastRayDown
  (bind _returnvalue (Transformation|GetActorLocation))
  (bind (_outhit _returnvalue_2) (Collision|LineTraceByChannel _returnvalue (- _returnvalue "0.000000,0.000000,2000.000000") "TraceTypeQuery2" false 0 "ForDuration"))
  (if _returnvalue_2
    (return (.Distance (Collision|BreakHitResult _outhit)) (.z (.Location (Collision|BreakHitResult _outhit))))
    (else
      (return 1e+04 0.0))))

(fn Hover
  (params (Hover%20Distance :type Float%20%28double-precision%29) (Force%20Intesnsity :type Float%20%28double-precision%29) (deltaTime :type Float%20%28double-precision%29))
  (bind _testcaragain (Variables|Default|Gettestcaragain))
  (bind _returnvalue (Transformation|GetWorldLocation _testcaragain))
  (bind _ground_z (CallFunction|CastRayDown))
  (Transformation|SetWorldLocation (Variables|Default|Gettestcaragain) (Math|Vector|MakeVector (.x _returnvalue) (.y _returnvalue) (Math|Interpolation|FInterpTo (.z _returnvalue) (+ Hover%20Distance _ground_z) deltaTime 2.0)) false false))

(fn AirResist
  (Variables|Default|SetCurrent%20Speed (select (> (Variables|Default|GetCurrent%20Speed) 0.0) (Math|Interpolation|FInterpTo (Variables|Default|GetCurrent%20Speed) (- (Variables|Default|GetCurrent%20Speed) (Variables|Default|GetAir%20Resist%20Constant)) (Utilities|Time|GetWorldDeltaSeconds) 3.0) (Math|Interpolation|FInterpTo (Variables|Default|GetCurrent%20Speed) (+ (Variables|Default|GetCurrent%20Speed) (Variables|Default|GetAir%20Resist%20Constant)) (Utilities|Time|GetWorldDeltaSeconds) 3.0))))

(fn SteerTilt
  (params (Angle :type Float%20%28double-precision%29))
  (bind _testcaragain (Variables|Default|Gettestcaragain))
  (bind _tiltdenom (Variables|Default|GetTiltDenom))
  (bind _returnvalue (Transformation|GetWorldRotation _testcaragain))
  (if (< _tiltdenom 3.0)
    (Development|PrintText "Sparks!" true true "(R=1.000000,G=0.937121,B=0.103198,A=1.000000)"))
  (Transformation|SetWorldRotation (Variables|Default|Gettestcaragain1) (Math|Rotator|MakeRotator (/ Angle _tiltdenom) (.pitch _returnvalue) (.yaw _returnvalue)) false false))

(fn LockPitch
  (bind _testcaragain (Variables|Default|Gettestcaragain))
  (bind _returnvalue (Transformation|GetWorldRotation _testcaragain))
  (Transformation|SetWorldRotation _testcaragain (Math|Rotator|MakeRotator (.roll _returnvalue) 0.0 (.yaw _returnvalue)) false false))

(fn SineOffset
  (params (Frequency :type Float%20%28double-precision%29) (Delta%20Time :type Float%20%28double-precision%29))
  (return (* 2.0 (Math|Trig|GetPI) Frequency Delta%20Time)))

(fn Sineify
  (params (Intensity :type Float%20%28double-precision%29) (InHoverPosit :type Float%20%28double-precision%29) (deltaTime :type Float%20%28double-precision%29))
  (bind _result (CallFunction|SineOffset 1e+01 deltaTime))
  (return (+ (* _result Intensity) InHoverPosit)))

(fn BindYaw
  (params (Steer%20Assist%20Value :type Float%20%28double-precision%29))
  (bind _spline (Variables|Default|GetSpline))
  (bind _testcaragain (Variables|Default|Gettestcaragain))
  (bind _returnvalue (Transformation|GetWorldRotation _testcaragain))
  (bind _spline_2 (Variables|/Game/Blueprints/Tracks/TestTrack.TestTrack_C|GetSpline _spline))
  (Transformation|SetWorldRotation (Variables|Default|Gettestcaragain) (Math|Rotator|MakeRotator (.roll _returnvalue) (.pitch _returnvalue) (Math|Interpolation|FInterpTo (.yaw _returnvalue) (.yaw (Spline|GetRotationatDistanceAlongSpline _spline_2 (Class|SplineComponent|GetDistanceAlongSplineatLocation _spline_2 (Transformation|GetWorldLocation (Variables|Default|Gettestcaragain)) "World") "World")) (Utilities|Time|GetWorldDeltaSeconds) Steer%20Assist%20Value)) false false))