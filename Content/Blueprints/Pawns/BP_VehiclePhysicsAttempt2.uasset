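; Player-driven hover vehicle pawn that moves a physics-simulated Model through Enhanced Input.
; Construction passes the Model and shared hover distance, force and damping to three hover components, which Tick snaps to front, back-left and back-right points.
; Thrust input eases speed into a forward force applied each Tick, while Turn input applies eased yaw torque.
; Roll torque and thrust location are computed but never applied, and Brake is empty.
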(event Input|EnhancedActionEvents|EnhancedInputActionThrust
  (params (ActionValue :type Float%20%28double-precision%29) (ElapsedSeconds :type Float%20%28double-precision%29) (TriggeredSeconds :type Float%20%28double-precision%29) (InputAction :type Input%20Action%20Object%20Reference :default "/Game/Controls/Thrust.Thrust"))
  (bind (_thrust_force _thrust_location) (CallFunction|Throttle ActionValue))
  (Variables|Thrust|SetThrustForce _thrust_force)
  (Variables|Thrust|SetThrustLoc _thrust_location))

(event Input|EnhancedActionEvents|EnhancedInputActionTurn
  (params (ActionValue :type Float%20%28double-precision%29) (ElapsedSeconds :type Float%20%28double-precision%29) (TriggeredSeconds :type Float%20%28double-precision%29) (InputAction :type Input%20Action%20Object%20Reference :default "/Game/Controls/Turn.Turn"))
  (bind (_ztorque _ytorque) (CallFunction|Turn ActionValue))
  (Variables|Steer|SetSteer%20Torque _ztorque)
  (Variables|Steer|SetRoll%20Torque _ytorque)
  (Class|PrimitiveComponent|AddTorqueinRadians (Variables|Default|GetModel) (* "0.000000,0.000000,1.000000" (Variables|Steer|GetSteer%20Torque)) "None" false))

(event EventBeginPlay
  (bind _asplayer_controller (Utilities|Casting|CastToPlayerController (Pawn|GetController)))
  (Utilities|IsValid (PlayerController|LocalPlayerSubsystems|GetEnhancedInputLocalPlayerSubsystem _asplayer_controller)
    (:Is%20Valid
      (Input|AddMappingContext (PlayerController|LocalPlayerSubsystems|GetEnhancedInputLocalPlayerSubsystem _asplayer_controller) "/Game/Controls/GameControls.GameControls" 0 "(bIgnoreAllPressedKeysUntilRelease=True,bForceImmediately=False,bNotifyUserSettings=False)"))))

(event Collision|EventActorBeginOverlap
  (params (OtherActor :type Actor%20Object%20Reference)))

(event EventTick
  (params (DeltaSeconds :type Float%20%28single-precision%29))
  (Variables|/Game/Blueprints/PhysicsComponents/AC_HoverComponent.AC_HoverComponent_C|SetLocation (Variables|Default|GetACHC_Front) (Transformation|GetWorldLocation (Variables|Default|GetHN%20Front)))
  (Variables|/Game/Blueprints/PhysicsComponents/AC_HoverComponent.AC_HoverComponent_C|SetLocation (Variables|Default|GetACHC_BackRIGHT) (Transformation|GetWorldLocation (Variables|Default|GetHN%20Back%20right)))
  (Variables|/Game/Blueprints/PhysicsComponents/AC_HoverComponent.AC_HoverComponent_C|SetLocation (Variables|Default|GetACHC_BackLEFT) (Transformation|GetWorldLocation (Variables|Default|GetHN%20Back%20left)))
  (Physics|AddForce (Variables|Default|GetModel) (Variables|Thrust|GetThrustForce) "None" false))

(fn ConstructionScript
  (CallFunction|BuildHoverArray)
  (CallFunction|SetHover))

(fn SetHover
  (for _array_element (Variables|Hover|GetHoverComponents)
    (Variables|/Game/Blueprints/PhysicsComponents/AC_HoverComponent.AC_HoverComponent_C|SetPrim _array_element (Variables|Default|GetModel))
    (Variables|/Game/Blueprints/PhysicsComponents/AC_HoverComponent.AC_HoverComponent_C|SetHover%20Distance _array_element (Variables|Hover|GetHoverDistance))
    (Variables|/Game/Blueprints/PhysicsComponents/AC_HoverComponent.AC_HoverComponent_C|SetForce _array_element (Variables|Hover|GetHoverForce))
    (Variables|/Game/Blueprints/PhysicsComponents/AC_HoverComponent.AC_HoverComponent_C|SetLinear%20Damping _array_element (Variables|Hover|GetLDamping))
    (Variables|/Game/Blueprints/PhysicsComponents/AC_HoverComponent.AC_HoverComponent_C|SetAngular%20Damping _array_element (Variables|Hover|GetADamping))))

(fn BuildHoverArray
  (Utilities|Array|Add (Variables|Hover|GetHoverComponents) (Variables|Default|GetACHC_Front))
  (Utilities|Array|Add (Variables|Hover|GetHoverComponents) (Variables|Default|GetACHC_BackLEFT))
  (Utilities|Array|Add (Variables|Hover|GetHoverComponents) (Variables|Default|GetACHC_BackRIGHT)))

(fn Throttle
  (params (ThrottleAxis :type Float%20%28double-precision%29))
  (bind _model (Variables|Default|GetModel))
  (bind _returnvalue (Transformation|GetWorldLocation _model))
  (bind _output_get (Variables|Throttle|SetCurrent%20Speed (Math|Interpolation|FInterpTo (Variables|Throttle|GetCurrent%20Speed) (* ThrottleAxis (Variables|Throttle|GetTop%20Speed)) (Utilities|Time|GetWorldDeltaSeconds) 3.5)))
  (return (* _output_get (Math|Vector|GetForwardVector (Variables|Default|GetModel))) (Math|Vector|MakeVector (.x _returnvalue) (.y _returnvalue) (- (.z _returnvalue) (Variables|Throttle|GetAccelZOffset)))))

(fn Turn
  (params (Turn%20Axis :type Float%20%28double-precision%29))
  (return (Math|Interpolation|FInterpTo (Variables|Steer|GetSteer%20Torque) (* Turn%20Axis (Variables|Steer|GetSteer%20Rad)) (Utilities|Time|GetWorldDeltaSeconds) 1e+01) (Math|Interpolation|FInterpTo (Variables|Steer|GetRoll%20Torque) (* Turn%20Axis (Variables|Steer|GetMax%20Roll%20Angle)) (Utilities|Time|GetWorldDeltaSeconds) 4.0)))

(fn Brake)