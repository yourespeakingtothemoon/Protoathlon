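; Physics-driven movement component that steers its owner toward a target forward speed and yaw rate.
; BeginPlay caches the root primitive, keeping it only if it simulates physics.
; Each tick, proportional control turns speed errors into forward force and torque about the up axis, plus scaled torque about the forward axis for banking.
; A speed-pitched thruster sound block exists but is disconnected and never runs.
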(event EventBeginPlay
  (bind _asprimitive_component (Utilities|Casting|CastToPrimitiveComponent (Variables|/Script/Engine.Actor|GetRootComponent (Components|GetOwner))))
  (bind _output_get (Variables|Default|SetBodyRef _asprimitive_component))
  (if (not (Physics|IsSimulatingPhysics _output_get "None"))
    (Variables|Default|SetBodyRef 0)))

(event EventTick
  (params (DeltaSeconds :type Float%20%28single-precision%29))
  (bind _turnsensitivity (Variables|Default|GetTurnSensitivity))
  (bind _bodyref (Variables|Default|GetBodyRef))
  (bind _bodyref_2 (Variables|Default|GetBodyRef))
  (bind _bodyref_3 (Variables|Default|GetBodyRef))
  (bind _bodyref_4 (Variables|Default|GetBodyRef))
  (bind _bodyref_5 (Variables|Default|GetBodyRef)
    (:then
      (bind _returnvalue (Physics|GetPhysicsLinearVelocity _bodyref_5 "None"))
      (Variables|Default|SetCurrentSpeed (Math|Vector|DotProduct _returnvalue (Math|Vector|GetForwardVector _bodyref_5)))
      (Variables|Default|SetCurrentAngularSpeed (Math|Vector|DotProduct (Physics|GetPhysicsAngularVelocityinDegrees _bodyref_2 "None") (Math|Vector|GetUpVector _bodyref_2)))
      (Physics|AddForce _bodyref_4 (* (Math|Vector|GetForwardVector _bodyref_4) (* (- (Variables|Default|GetTargetSpeed) (Variables|Default|GetCurrentSpeed)) (Variables|Default|GetAccelerationFactor))) "None" false)
      (Class|PrimitiveComponent|AddTorqueinDegrees _bodyref (* (Math|Vector|GetUpVector _bodyref) (* (- (Variables|Default|GetTargetAngularSpeed) (Variables|Default|GetCurrentAngularSpeed)) _turnsensitivity)) "None" false)
      (Class|PrimitiveComponent|AddTorqueinDegrees _bodyref_3 (* (Math|Vector|GetForwardVector _bodyref_3) (/ (* (- (Variables|Default|GetTargetAngularSpeed) (Variables|Default|GetCurrentAngularSpeed)) _turnsensitivity) (Variables|Default|Getroll%20numerator))) "None" false))
    (:else)))