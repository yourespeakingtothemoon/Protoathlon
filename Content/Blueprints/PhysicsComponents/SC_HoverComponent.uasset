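; Scene component that acts as a raycast hover spring, pushing its owner's physics-simulating root body away from surfaces below the component.
; Each tick it traces along its own down vector up to HoverDistance and converts the hit into a normalized compression.
; A spring term plus a damping term from the compression's rate of change sets the force, applied along the body's up vector at the component's location.
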(event EventBeginPlay
  (bind _asprimitive_component (Utilities|Casting|CastToPrimitiveComponent (Variables|/Script/Engine.Actor|GetRootComponent (Components|GetOwner))))
  (bind _output_get (Variables|Default|SetBodyRef _asprimitive_component))
  (if (not (Physics|IsSimulatingPhysics _output_get "None"))
    (Variables|Default|SetBodyRef 0)))

(event EventTick
  (params (DeltaSeconds :type Float%20%28single-precision%29))
  (Variables|Default|GetBodyRef
    (:then
      (CallFunction|SuspensionTrace))
    (:else)))

(fn SuspensionTrace
  (bind _returnvalue (Transformation|GetWorldLocation))
  (bind _bodyref (Variables|Default|GetBodyRef))
  (bind (_outhit _returnvalue_2) (Collision|LineTraceByChannel _returnvalue (- _returnvalue (* (Math|Vector|GetUpVector) (Variables|Default|GetHover%20Distance))) "TraceTypeQuery1" false (Utilities|Array|MakeArray (Components|GetOwner)) (select (Variables|Default|GetdebugRaycast) "ForOneFrame" "None")))
  (Variables|Default|Setis%20hit _returnvalue_2)
  (if _returnvalue_2
    (Variables|Default|SetHover%20Force (+ (* (/ (- (/ (- (Variables|Default|GetHover%20Distance) (.Distance (Collision|BreakHitResult _outhit))) (Variables|Default|GetHover%20Distance)) (Variables|Default|GetPrevious%20Compression%20Offset)) (Utilities|Time|GetWorldDeltaSeconds)) (Variables|Default|GetDamping%20Factor)) (* (/ (- (Variables|Default|GetHover%20Distance) (.Distance (Collision|BreakHitResult _outhit))) (Variables|Default|GetHover%20Distance)) (Variables|Default|GetSuspension%20Force%20Factor))))
    (Variables|Default|SetPrevious%20Compression%20Offset (/ (- (Variables|Default|GetHover%20Distance) (.Distance (Collision|BreakHitResult _outhit))) (Variables|Default|GetHover%20Distance)))
    (Class|PrimitiveComponent|AddForceatLocation _bodyref (* (Math|Vector|GetUpVector _bodyref) (Variables|Default|GetHover%20Force)) (Transformation|GetWorldLocation) "None")))