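; Player vehicle pawn that uses Enhanced Input for thrust and turn, and snaps its car mesh to the ground.
; Each tick, steer input accumulates into yaw, while a downward trace sets height and tilts the mesh to the surface normal.
; Thrust interpolates a current speed, but the forward force is multiplied by zero, so speed never drives movement.
; BeginPlay also caches the TestTrack actor as Spline, which is otherwise unused.
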(event Input|EnhancedActionEvents|EnhancedInputActionThrust
  (params (ActionValue :type Float%20%28double-precision%29) (ElapsedSeconds :type Float%20%28double-precision%29) (TriggeredSeconds :type Float%20%28double-precision%29) (InputAction :type Input%20Action%20Object%20Reference :default "/Game/Controls/Thrust.Thrust"))
  (bind _speed (CallFunction|Throttle ActionValue (Variables|Default|GetMax%20Speed)))
  (Variables|Default|SetCurrent%20Speed _speed))

(event Input|EnhancedActionEvents|EnhancedInputActionTurn
  (params (ActionValue :type Float%20%28double-precision%29) (ElapsedSeconds :type Float%20%28double-precision%29) (TriggeredSeconds :type Float%20%28double-precision%29) (InputAction :type Input%20Action%20Object%20Reference :default "/Game/Controls/Turn.Turn"))
  (Variables|Default|SetCurrent%20Steer%20Angle ActionValue))

(event EventBeginPlay
  (bind _asplayer_controller (Utilities|Casting|CastToPlayerController (Pawn|GetController)))
  (Utilities|IsValid (PlayerController|LocalPlayerSubsystems|GetEnhancedInputLocalPlayerSubsystem _asplayer_controller)
    (:Is%20Valid
      (Input|AddMappingContext (PlayerController|LocalPlayerSubsystems|GetEnhancedInputLocalPlayerSubsystem _asplayer_controller) "/Game/Controls/GameControls.GameControls" 0 "(bIgnoreAllPressedKeysUntilRelease=True,bForceImmediately=False,bNotifyUserSettings=False)")
      (bind _returnvalue (Actor|GetActorOfClass "/Game/Blueprints/Tracks/TestTrack.TestTrack_C"))
      (Variables|Default|SetSpline _returnvalue))))

(event Collision|EventActorBeginOverlap
  (params (OtherActor :type Actor%20Object%20Reference)))

(event EventTick
  (params (DeltaSeconds :type Float%20%28single-precision%29))
  (CallFunction|UpdateMovement)
  (CallFunction|UpdatePhysics))

(fn ConstructionScript)

(fn UpdateMovement
  (Physics|AddForce (Variables|Default|Gettestcaragain) (* (Transformation|GetActorForwardVector) 0.0) "None" false)
  (Variables|Default|SetAngle (+ (Variables|Default|GetAngle) (Variables|Default|GetCurrent%20Steer%20Angle))))

(fn UpdatePhysics
  (bind _newparam (CallFunction|CastRayDown))
  (Transformation|SetWorldLocationAndRotation (Variables|Default|Gettestcaragain) (Math|Vector|MakeVector (.X (Math|Vector|BreakVector (.Location (Collision|BreakHitResult _newparam)))) (.Y (Math|Vector|BreakVector (.Location (Collision|BreakHitResult _newparam)))) (+ (.Z (Math|Vector|BreakVector (.Location (Collision|BreakHitResult _newparam)))) 16.0)) (Math|Rotator|MakeRotator (.Roll (Math|Rotator|BreakRotator (Math|Rotator|MakeRotfromZX (.ImpactNormal (Collision|BreakHitResult _newparam)) (Transformation|GetActorForwardVector)))) (.Pitch (Math|Rotator|BreakRotator (Math|Rotator|MakeRotfromZX (.ImpactNormal (Collision|BreakHitResult _newparam)) (Transformation|GetActorForwardVector)))) (Variables|Default|GetAngle)) false false))

(fn Throttle
  (params (Throttle%20Amount :type Float%20%28double-precision%29) (Max%20Speed :type Float%20%28double-precision%29))
  (return (Math|Interpolation|FInterpTo (Variables|Default|GetCurrent%20Speed) (* Throttle%20Amount Max%20Speed) (Utilities|Time|GetWorldDeltaSeconds) 4.0)))

(fn CastRayDown
  (bind _returnvalue (Transformation|GetActorLocation))
  (bind (_outhit _returnvalue_2) (Collision|LineTraceByChannel _returnvalue (- _returnvalue "0.000000,0.000000,2000.000000") "TraceTypeQuery2" false 0 "ForDuration"))
  (if _returnvalue_2
    (return (.Distance (Collision|BreakHitResult _outhit)) (.z (.Location (Collision|BreakHitResult _outhit))) _outhit)
    (else
      (return 1e+04 0.0 ""))))